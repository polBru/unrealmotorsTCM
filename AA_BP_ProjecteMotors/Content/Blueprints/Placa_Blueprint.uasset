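; Placa Blueprint is an actor that cycles its point light through three configurable colors each time another actor overlaps it.
; On BeginPlay it fills a color array from three color variables and sets the light to the first one.
; Each overlap advances an index that wraps back to zero after the third color, then applies that array entry to the light.
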(event `self.ReceiveBeginPlay`
  (`KismetArrayLibrary.Array_Set` (`self.ColorArray`) 0 (`self.Color1`) true)
  (`KismetArrayLibrary.Array_Set` (`self.ColorArray`) 1 (`self.Color2`) true)
  (`KismetArrayLibrary.Array_Set` (`self.ColorArray`) 2 (`self.Color3`) true)
  (`LightComponent.SetLightColor` (`self.PointLight`) (`KismetMathLibrary.Conv_ColorToLinearColor` (`self.Color1`)) true))

(event `self.ReceiveActorBeginOverlap`
  (params (OtherActor :type "Actor Object Reference"))
  (if (<= (`self.CurrentPoition`) 1)
    (set `self.CurrentPoition` (+ (`self.CurrentPoition`) 1))
    (else
      (set `self.CurrentPoition` 0)))
  (`LightComponent.SetLightColor` (`self.PointLight`) (`KismetMathLibrary.Conv_ColorToLinearColor` (`|GetArrayItem` (`self.ColorArray`) (`self.CurrentPoition`))) true))

(event `self.ReceiveTick`
  (params (DeltaSeconds :type "Float (single-precision)")))

(fn `UserConstructionScript`)