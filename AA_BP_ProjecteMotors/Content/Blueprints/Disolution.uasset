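; Actor Blueprint that dissolves its static mesh with a burn effect when T is pressed, then destroys itself.
; On BeginPlay it creates a dynamic material instance from the mesh's first material slot.
; The key press enables the AllowBurn parameter and plays a timeline that drives DisolutionValue at half the track value.
; When the timeline finishes, the actor is destroyed.
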(event `self.ReceiveBeginPlay`
  (bind _returnvalue (`KismetMaterialLibrary.CreateDynamicMaterialInstance` (`|GetArrayItem` (`MeshComponent.GetMaterials` (`self.StaticMesh`)))))
  (`PrimitiveComponent.SetMaterial` (`self.StaticMesh`) 0 _returnvalue))

(event `Key|T`
  (params (Key :type "Key Structure"))
  (bind _staticmesh (`self.StaticMesh`))
  (:`Pressed`
    (`MeshComponent.SetScalarParameterValueOnMaterials` _staticmesh "AllowBurn" 1.0)
    (bind (_direction _newtrack_0) (`Timeline|Timeline_0`)
      (:`Update`
        (`MeshComponent.SetScalarParameterValueOnMaterials` _staticmesh "DisolutionValue" (/ _newtrack_0 2.0)))
      (:`Finished`
        (`self.K2_DestroyActor`)))))

(fn `UserConstructionScript`)