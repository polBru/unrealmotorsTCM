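; Key pickup actor that bobs up and down and spins in place until something overlaps it.
; BeginPlay stores the starting height, then Tick offsets Z from it with a degree-based sine wave and advances yaw, resetting the angle after a full turn.
; Any actor overlap sets HasKey to true, with no filtering of the other actor and no hiding or destroying of the key.
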(event `self.ReceiveBeginPlay`
  (bind (_returnvalue_x _returnvalue_y _returnvalue_z) (`KismetMathLibrary.BreakVector` (`self.K2_GetActorLocation`)))
  (set `self.ReferenceHeight` _returnvalue_z))

(event `self.ReceiveTick`
  (params (DeltaSeconds :type "Float (single-precision)"))
  (bind (_returnvalue_x _returnvalue_y) (`KismetMathLibrary.BreakVector` (`self.K2_GetActorLocation`)))
  (set `self.T` (+ (`self.T`) (* (`self.SpeedSinus`) DeltaSeconds)))
  (set `self.Angle` (+ (`self.Angle`) (* (`self.RotationSpeed`) DeltaSeconds)))
  (`self.K2_SetActorLocation` (`KismetMathLibrary.MakeVector` _returnvalue_x _returnvalue_y (+ (`self.ReferenceHeight`) (* (`self.Amplitude`) (`KismetMathLibrary.DegSin` (`self.T`))))))
  (`self.K2_SetActorRotation` (`KismetMathLibrary.MakeRotator` 0.0 0.0 (`self.Angle`)))
  (if (>= (`self.Angle`) 360.0)
    (set `self.Angle` 0.0)))

(event `self.ReceiveActorBeginOverlap`
  (params (OtherActor :type "Actor Object Reference"))
  (set `self.HasKey` true))

(fn `UserConstructionScript`)