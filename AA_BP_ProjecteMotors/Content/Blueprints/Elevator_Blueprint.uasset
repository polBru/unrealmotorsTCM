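; Elevator actor that rises by a set Elevation when any actor overlaps it and returns to its start when an overlap ends.
; BeginPlay stores the starting location and the raised location as two waypoints, and the overlap events switch the current target between them.
; Tick lerps the actor toward that target by DeltaSeconds times Speed, giving an ease-out motion without sweep collision.
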(event `self.ReceiveBeginPlay`
  (bind (_returnvalue_x _returnvalue_y _returnvalue_z) (`KismetMathLibrary.BreakVector` (`self.K2_GetActorLocation`)))
  (`KismetArrayLibrary.Array_Set` (`self.WayPoints`) 0 (`self.K2_GetActorLocation`) true)
  (`KismetArrayLibrary.Array_Set` (`self.WayPoints`) 1 (`KismetMathLibrary.MakeVector` _returnvalue_x _returnvalue_y (+ _returnvalue_z (`self.Elevation`))) true))

(event `self.ReceiveActorBeginOverlap`
  (params (OtherActor :type "Actor Object Reference"))
  (set `self.CurrentPoint` 1))

(event `self.ReceiveActorEndOverlap`
  (params (OtherActor :type "Actor Object Reference"))
  (set `self.CurrentPoint` 0))

(event `self.ReceiveTick`
  (params (DeltaSeconds :type "Float (single-precision)"))
  (if (!= (`self.K2_GetActorLocation`) (`|GetArrayItem` (`self.WayPoints`) (`self.CurrentPoint`)))
    (`self.K2_SetActorLocation` (`KismetMathLibrary.VLerp` (`self.K2_GetActorLocation`) (`|GetArrayItem` (`self.WayPoints`) (`self.CurrentPoint`)) (* DeltaSeconds (`self.Speed`))))))

(fn `UserConstructionScript`)