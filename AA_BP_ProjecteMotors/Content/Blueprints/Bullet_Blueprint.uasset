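; Bullet actor that transfers player control to an agent it overlaps, acting as a possession shot.
; On overlapping an actor of exactly the Agent_Blueprint class, it sets that agent's state to 1, flags it as possessed and has player controller 0 possess it.
; The bullet then destroys itself, or expires ten seconds after spawning if it overlaps no agent.
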(event `self.ReceiveHit`
  (params (MyComp :type "PrimitiveComponent Object Reference") (Other :type "Actor Object Reference") (OtherComp :type "PrimitiveComponent Object Reference") (bSelfMoved :type Boolean) (HitLocation :type "Vector Structure") (HitNormal :type "Vector Structure") (NormalImpulse :type "Vector Structure") (Hit :type "HitResult Structure (by ref)")))

(event `self.ReceiveActorBeginOverlap`
  (params (OtherActor :type "Actor Object Reference"))
  (if (== (`GameplayStatics.GetObjectClass` OtherActor) "/Game/Blueprints/Agent_Blueprint.Agent_Blueprint_C")
    (bind _asagent_blueprint (cast `/Game/Blueprints/Agent_Blueprint` OtherActor))
    (bind (_agenttransform _state _currentposition _health) (break `/Game/Blueprints/AgentStruct` (`/Game/Blueprints/Agent_Blueprint.AgentVariables` _asagent_blueprint)))
    (set `/Game/Blueprints/Agent_Blueprint.AgentVariables` (make `/Game/Blueprints/AgentStruct` _agenttransform 1 _currentposition _health) _asagent_blueprint)
    (set `/Game/Blueprints/Agent_Blueprint.possessed` true _asagent_blueprint)
    (`Controller.Possess` (`GameplayStatics.GetPlayerController` 0) _asagent_blueprint)
    (`self.K2_DestroyActor`)))

(event `self.ReceiveBeginPlay`
  (`KismetSystemLibrary.Delay` 10.0)
  (`self.K2_DestroyActor`))

(fn `UserConstructionScript`)