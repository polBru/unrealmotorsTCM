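; Door actor that rises when the third-person character overlaps it and lowers when an overlap ends.
; A door type selects the opening condition: none, enough coins, a key, or a completed puzzle.
; Failed coin and key checks show a hint on a text render, hidden again on overlap end.
; Tick lerps the actor toward the raised or initial position using delta time and speed, giving an eased slide.
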(event `self.ReceiveActorBeginOverlap`
  (params (OtherActor :type "Actor Object Reference"))
  (bind _textrender (`self.TextRender`))
  (bind _textrender_2 (`self.TextRender`))
  (if (== (`GameplayStatics.GetObjectClass` OtherActor) "/Game/ThirdPersonBP/Blueprints/ThirdPersonCharacter.ThirdPersonCharacter_C")
    (if (== (`self.TypeOfDoor`) 0)
      (set `self.Open` true)
      (elif (== (`self.TypeOfDoor`) 1)
        (if (`self.HasMinimumCoins`)
          (set `self.Open` true)
          (else
            (bind _output_get (set `self.SplashText` "No Enough Coins"))
            (`TextRenderComponent.K2_SetText` _textrender _output_get)
            (`SceneComponent.SetVisibility` _textrender true false)))
        (elif (== (`self.TypeOfDoor`) 2)
          (if (`self.HasKey`)
            (set `self.Open` true)
            (else
              (bind _output_get_2 (set `self.SplashText` "Need the key"))
              (`TextRenderComponent.K2_SetText` _textrender_2 _output_get_2)
              (`SceneComponent.SetVisibility` _textrender_2 true false)))
          (elif (`self.IsPuzzleCompleted`)
            (set `self.Open` true)))))))

(event `self.ReceiveActorEndOverlap`
  (params (OtherActor :type "Actor Object Reference"))
  (set `self.Open` false)
  (`SceneComponent.SetVisibility` (`self.TextRender`) false false))

(event `self.ReceiveBeginPlay`
  (bind (_returnvalue_x _returnvalue_y _returnvalue_z) (`KismetMathLibrary.BreakVector` (`self.K2_GetActorLocation`)))
  (set `self.InitialPos` (`self.K2_GetActorLocation`))
  (set `self.UpPos` (`KismetMathLibrary.MakeVector` _returnvalue_x _returnvalue_y (+ _returnvalue_z (`self.Elevation`)))))

(event `self.ReceiveTick`
  (params (DeltaSeconds :type "Float (single-precision)"))
  (if (`self.Open`)
    (`self.K2_SetActorLocation` (`KismetMathLibrary.VLerp` (`self.K2_GetActorLocation`) (`self.UpPos`) (* DeltaSeconds (`self.Speed`))))
    (else
      (`self.K2_SetActorLocation` (`KismetMathLibrary.VLerp` (`self.K2_GetActorLocation`) (`self.InitialPos`) (* DeltaSeconds (`self.Speed`)))))))

(fn `UserConstructionScript`)